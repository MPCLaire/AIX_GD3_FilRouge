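; Row actor for a Mastermind game, holding four answer sphere references and responding to mouse clicks.
; On BeginPlay it gathers its four spheres into the AnswerSpheres array.
; A click on the actor is forwarded to Clicked, whose logic is not defined in these graphs.
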(event `self.ReceiveBeginPlay`
  (`KismetArrayLibrary.Array_Add` (`self.AnswerSpheres`) (`self.Sphere1`))
  (`KismetArrayLibrary.Array_Add` (`self.AnswerSpheres`) (`self.Sphere2`))
  (`KismetArrayLibrary.Array_Add` (`self.AnswerSpheres`) (`self.Sphere3`))
  (`KismetArrayLibrary.Array_Add` (`self.AnswerSpheres`) (`self.Sphere`)))

(event `self.ReceiveActorOnClicked`
  (params (ButtonPressed :type "Key Structure"))
  (`self.Clicked`))

(fn `UserConstructionScript`)